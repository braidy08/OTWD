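; Mod actor that shows a health bar widget for the AI character the local player is looking at.
; BeginPlay creates the widget, then retries every 0.2 seconds until it gets the player pawn, repeating setup when that pawn is destroyed.
; A looping timer line-traces forward from the first-person camera attachment, feeding a hit AI's health attributes to the widget or hiding it otherwise.
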(event Custom|OnDestroyed_Event_0
  (params (DestroyedActor :type Actor%20Object%20Reference))
  (bind _menu_healthbar (Variables|Default|GetMenu_HealthBar))
  (bind _assbzplayer_character (Utilities|Casting|CastToSBZPlayerCharacter (Class|SBZUtility|GetLocalPlayerPawn) :!label _label)
    (:then
      (bind _output_get (Variables|Default|SetAs%20SBZPlayer%20Character _assbzplayer_character))
      (Variables|Default|SetFPCamera%20Attachment (Variables|/Script/Starbreeze.SBZPlayerCharacter|GetFPCameraAttachment _output_get))
      (Utilities|Time|SetTimerbyEvent (delegate Custom|CustomEvent_0) 0.0 true)
      (Widget|SetVisibility (Variables|Default|GetMenu_HealthBar) "Collapsed")
      (Game|BindEventtoOnDestroyed (Variables|Default|GetAs%20SBZPlayer%20Character) (delegate Custom|OnDestroyed_Event_0)))
    (:CastFailed
      (Default|SetText _menu_healthbar "SBZPlayer Casting Failed")
      (Widget|SetVisibility _menu_healthbar "Collapsed")
      (Utilities|FlowControl|Delay 0.2)
      (goto _label))))

(event Custom|CustomEvent_0
  (bind _fpcamera_attachment (Variables|Default|GetFPCamera%20Attachment))
  (bind _returnvalue (Transformation|GetWorldLocation _fpcamera_attachment))
  (bind (_outhit _returnvalue_2) (Collision|LineTraceByChannel _returnvalue (+ _returnvalue (* (Math|Vector|GetForwardVector _fpcamera_attachment) 3e+04)) "TraceTypeQuery2" false (Utilities|Array|MakeArray (Variables|Default|GetAs%20SBZPlayer%20Character)) "None"))
  (if _returnvalue_2
    (if (Utilities|ClassIsChildOf (Utilities|GetClass (.HitActor (Collision|BreakHitResult _outhit))) "/Script/Starbreeze.SBZAICharacter")
      (bind _assbzaicharacter (Utilities|Casting|CastToSBZAICharacter (.HitActor (Collision|BreakHitResult _outhit)))
        (:then
          (Widget|SetVisibility (Variables|Default|GetMenu_HealthBar) "SelfHitTestInvisible")
          (Default|SetHealth (Variables|Default|GetMenu_HealthBar) (Variables|/Script/Starbreeze.SBZHealthAttributeSet|GetHealth (Variables|/Script/Starbreeze.SBZCharacter|GetHealthAttributeSet _assbzaicharacter)) (Variables|/Script/Starbreeze.SBZHealthAttributeSet|GetHealthMaximum (Variables|/Script/Starbreeze.SBZCharacter|GetHealthAttributeSet _assbzaicharacter))))
        (:CastFailed
          (Widget|SetVisibility (Variables|Default|GetMenu_HealthBar) "Hidden" :!label _label)))
      (else
        (goto _label)))
    (else
      (goto _label))))

(event EventBeginPlay
  (|CallParentFunction)
  (bind _returnvalue (UserInterface|CreateWidget "/Game/Mods/SimpleHealthHudTest/Menu_SimpleHealthBar.Menu_SimpleHealthBar_C"))
  (UserInterface|Viewport|AddtoViewport _returnvalue 0)
  (Variables|Default|SetMenu_HealthBar _returnvalue)
  (Widget|SetVisibility (Variables|Default|GetMenu_HealthBar) "Collapsed")
  (bind _assbzplayer_character (Utilities|Casting|CastToSBZPlayerCharacter (Class|SBZUtility|GetLocalPlayerPawn) :!label _label)
    (:then
      (bind _output_get (Variables|Default|SetAs%20SBZPlayer%20Character _assbzplayer_character))
      (Variables|Default|SetFPCamera%20Attachment (Variables|/Script/Starbreeze.SBZPlayerCharacter|GetFPCameraAttachment _output_get))
      (Utilities|Time|SetTimerbyEvent (delegate Custom|CustomEvent_0) 0.0 true)
      (Widget|SetVisibility (Variables|Default|GetMenu_HealthBar) "Collapsed")
      (Game|BindEventtoOnDestroyed (Variables|Default|GetAs%20SBZPlayer%20Character) (delegate Custom|OnDestroyed_Event_0)))
    (:CastFailed
      (Default|SetText (Variables|Default|GetMenu_HealthBar) "SBZPlayer Casting Failed")
      (Widget|SetVisibility (Variables|Default|GetMenu_HealthBar) "Collapsed")
      (Utilities|FlowControl|Delay 0.2)
      (goto _label))))

(fn ConstructionScript
  (|CallParentFunction))